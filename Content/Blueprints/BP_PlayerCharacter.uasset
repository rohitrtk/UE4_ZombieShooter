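; BP_PlayerCharacter is the player character Blueprint, handling HUD setup and a pause menu toggle.
; BeginPlay creates the player HUD widget and adds it to the viewport.
; PauseGame pauses with a cached in-game menu, created on first use, switching to UI-only input with a locked, visible cursor.
; Unpausing removes all widgets, rebuilds the HUD and restores game-only input with a hidden cursor.
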(event `SetupPlayerHUD`
  (bind _returnvalue (`|CreateWidget` "/Game/Blueprints/Widget/WBP_PlayerHUD.WBP_PlayerHUD_C"))
  (`UserWidget.AddToViewport` _returnvalue 0))

(event `self.ReceiveBeginPlay`
  (`self.SetupPlayerHUD`))

(event `self.PauseGame`
  (bind _returnvalue (`GameplayStatics.GetPlayerController` 0))
  (bind _returnvalue_2 (`GameplayStatics.GetPlayerController` 0))
  (if (`GameplayStatics.IsGamePaused`)
    (`GameplayStatics.SetGamePaused` false)
    (`WidgetLayoutLibrary.RemoveAllWidgets`)
    (`self.SetupPlayerHUD`)
    (`WidgetBlueprintLibrary.SetInputMode_GameOnly` _returnvalue)
    (set `PlayerController.bShowMouseCursor` false _returnvalue)
    (else
      (`GameplayStatics.SetGamePaused` true)
      (`/Engine/EditorBlueprintResources/StandardMacros.IsValid` (`self.InGameMenu`)
        (:`Is Valid`
          _)
        (:`Is Not Valid`
          (bind _returnvalue_3 (`|GenericCreateObject` "/Game/Blueprints/Widget/WBP_InGameMenu.WBP_InGameMenu_C" _returnvalue_2))
          (bind _output_get (set `self.InGameMenu` _returnvalue_3))))
      (`UserWidget.AddToViewport` _output_get 0)
      (`WidgetBlueprintLibrary.SetInputMode_UIOnlyEx` _returnvalue_2 (`self.InGameMenu`) "LockAlways")
      (set `PlayerController.bShowMouseCursor` true _returnvalue_2))))

(fn `UserConstructionScript`)